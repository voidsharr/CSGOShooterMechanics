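; AK-47 weapon Blueprint handling hitscan firing, ammo and reloading.
; Fire runs single shots or a gated retriggerable-delay loop for automatic mode, which StopFire closes and which adds random spread affected by movement and ADS.
; Muzzle line traces apply damage and choose impact effects by component tag, alongside muzzle flash, sound, camera shake and procedural arm recoil.
; Reload checks ammo, plays arm and rifle montages, then clears the reload state after a delay.
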(event `self.Fire`
  (bind (_initial _final) (`self.SimpleTrace`))
  (bind _asfp_character (`self.Cast`))
  (bind _returnvalue (`KismetMathLibrary.RandomFloatInRange` 1.0 1.2))
  (bind _returnvalue_2 (`GameplayStatics.GetPlayerController` 0))
  (bind _impact_point (`self.Impact Point`))
  (bind _returnvalue_3 (`SceneComponent.K2_GetComponentLocation` (`self.Muzzle`)))
  (bind _returnvalue_4 (+ _returnvalue 2.0))
  (bind _returnvalue_5 (select `bool` (`self.FiremodeCheck` "NewEnumerator1") :`false` _final :`true` (select `bool` (> (`KismetMathLibrary.VSize` (`CharacterMovementComponent.GetLastUpdateVelocity` (`Character.CharacterMovement` (`self.Cast`)))) 0.0) :`false` (`self.SpreadTrace` _final -5.0) :`true` (`self.SpreadTrace` _final -9.0))))
  (if (not (or (`/Game/GameContent/Blueprints/FPCharacter/FP_Character.Reload` _asfp_character) (`/Game/GameContent/Blueprints/FPCharacter/FP_Character.Run` _asfp_character)))
    (if (`self.FiremodeCheck` "NewEnumerator1")
      (`|ExecutionSequence`
        (:`then_0`
          (goto _label :!via `Open`))
        (:`then_1`
          (`/Engine/EditorBlueprintResources/StandardMacros.Gate` true :!label _label
            (:`Exit`
              (`|ExecutionSequence`
                (:`then_0`
                  (`KismetSystemLibrary.RetriggerableDelay` 0.1)
                  (goto _label))
                (:`then_1`
                  _)))))))
    (`self.F_AmmoCheck`
      (:`True`
        (`KismetSystemLibrary.PrintString` (`KismetStringLibrary.Conv_VectorToString` _returnvalue_5) true true (struct :`R` 1.0 :`G` 0.039628 :`A` 1.0) 3.0)
        (bind (_outhit _returnvalue_6) (`KismetSystemLibrary.LineTraceSingle` _initial _returnvalue_5 "TraceTypeQuery1"))
        (if _returnvalue_6
          (bind (_bblockinghit _binitialoverlap _time _distance _location _impactpoint _normal _impactnormal _physmat _hitactor _hitcomponent) (`GameplayStatics.BreakHitResult` _outhit))
          (bind _output_get (set `self.Impact Point` _impactpoint))
          (`KismetSystemLibrary.PrintString` (`KismetStringLibrary.Conv_VectorToString` _output_get))
          (`GameplayStatics.ApplyDamage` _hitactor 50.0 null (`self.Cast`))
          (`|ExecutionSequence`
            (:`then_0`
              (`GameplayStatics.SpawnEmitterAtLocation` "/Game/MilitaryWeapDark/FX/P_AssaultRifle_MuzzleFlash.P_AssaultRifle_MuzzleFlash" (`SceneComponent.K2_GetComponentLocation` (`self.Muzzle`)) (struct :`Yaw` 90.0) :!label _label_2)
              (if (`self.FiremodeCheck` "NewEnumerator0")
                (`GameplayStatics.PlaySoundAtLocation` "/Game/GameContent/Sounds/CAK/Rifle_CAK_Fire.Rifle_CAK_Fire" _returnvalue_3 (struct) _returnvalue_4 _returnvalue 0.0 "/Game/MilitaryWeapDark/Sound/Attenuation/WeaponShot_att.WeaponShot_att" null null null)
                (`PlayerController.ClientStartCameraShake` :`self` _returnvalue_2 :`Shake` "/Game/GameContent/CameraShakes/CS_Fire_Single.CS_Fire_Single_C")
                (else
                  (`PlayerController.ClientStartCameraShake` :`self` _returnvalue_2 :`Shake` "/Game/GameContent/CameraShakes/CS_Fire_Full.CS_Fire_Full_C")
                  (`GameplayStatics.PlaySoundAtLocation` "/Game/GameContent/Sounds/CAK/Rifle_CAK_Fire.Rifle_CAK_Fire" _returnvalue_3 (struct) _returnvalue_4 _returnvalue 0.0 "/Game/MilitaryWeapDark/Sound/Attenuation/WeaponShotClose_Att.WeaponShotClose_Att" null null null)))
              (`/Game/GameContent/Blueprints/FPCharacter/ABP_FPArms.ProceduralRecoil` (`/Game/GameContent/Blueprints/FPCharacter/FP_Character.As ABP FPArms` (`self.Cast`)) 0.5))
            (:`then_1`
              (if (`ActorComponent.ComponentHasTag` _hitcomponent "Wood")
                (`GameplayStatics.SpawnEmitterAtLocation` "/Game/MilitaryWeapDark/FX/P_Impact_Wood_Large_01.P_Impact_Wood_Large_01" _impact_point)
                (`GameplayStatics.PlaySoundAtLocation` "/Game/GameContent/Sounds/Wood.Wood" _impact_point (struct) 1.0 1.0 0.0 "/Game/MilitaryWeapDark/Sound/Attenuation/ProjectileImpact_att.ProjectileImpact_att" null null null)
                (elif (`ActorComponent.ComponentHasTag` _hitcomponent "Metal")
                  (`GameplayStatics.SpawnEmitterAtLocation` "/Game/MilitaryWeapDark/FX/P_Impact_Metal_Large_01.P_Impact_Metal_Large_01" _impact_point)
                  (`GameplayStatics.PlaySoundAtLocation` "/Game/GameContent/Sounds/Metal.Metal" _impact_point (struct) 1.0 1.0 0.0 "/Game/MilitaryWeapDark/Sound/Attenuation/ProjectileImpact_att.ProjectileImpact_att" null null null)
                  (elif (`ActorComponent.ComponentHasTag` _hitcomponent "Stone")
                    (`GameplayStatics.SpawnEmitterAtLocation` "/Game/MilitaryWeapDark/FX/P_Impact_Stone_Large_01.P_Impact_Stone_Large_01" _impact_point)
                    (`GameplayStatics.PlaySoundAtLocation` "/Game/MilitaryWeapDark/Sound/Rifle/Wavs/Rifle_ImpactSurface03.Rifle_ImpactSurface03" _impact_point (struct) 1.0 1.0 0.0 "/Game/MilitaryWeapDark/Sound/Attenuation/ProjectileImpact_att.ProjectileImpact_att" null null null)
                    (else
                      (`GameplayStatics.SpawnEmitterAtLocation` null _impact_point)
                      (`GameplayStatics.PlaySoundAtLocation` "/Game/GameContent/Sounds/Grass.Grass" _impact_point (struct) 1.0 1.0 0.0 "/Game/MilitaryWeapDark/Sound/Attenuation/ProjectileImpact_att.ProjectileImpact_att" null null null)))))))
          (else
            (goto _label_2)))))))

(event `StopFire`
  (goto _label :!via `Close`))

(event `self.Reload`
  (bind _asfp_character (`self.Cast`))
  (bind _asfp_character_2 (`self.Cast`))
  (if (not (or (`/Game/GameContent/Blueprints/FPCharacter/FP_Character.Reload` _asfp_character_2) (`/Game/GameContent/Blueprints/FPCharacter/FP_Character.Fire` _asfp_character_2)))
    (`self.R_AmmoCheck`
      (:`Check`
        (set `/Game/GameContent/Blueprints/FPCharacter/FP_Character.Reload` true _asfp_character)
        (`|PlayMontage` (`/Game/GameContent/Blueprints/FPCharacter/FP_Character.ArmsMesh` (`self.Cast`)) "/Game/GameContent/Animations/FPArms/Arm_RifleReload_Montage.Arm_RifleReload_Montage"
          (:`then`
            (`|PlayMontage` (`self.SkeletalMesh`) "/Game/GameContent/Animations/CAK/Rifle_Reload_Montage.Rifle_Reload_Montage"
              (:`then`
                (`KismetSystemLibrary.Delay` (`self.ReloadTime`))
                (set `/Game/GameContent/Blueprints/FPCharacter/FP_Character.Reload` false (`self.Cast`)))))))
      (:`false`
        (set `/Game/GameContent/Blueprints/FPCharacter/FP_Character.Reload` false _asfp_character)))))

(fn `AudioRandom`
  (params (Min :type "Float (double-precision)") (Max :type "Float (double-precision)"))
  (returns (`1st` :type "Float (double-precision)") (`2nd` :type "Float (double-precision)"))
  (bind _returnvalue (`KismetMathLibrary.RandomFloatInRange` Min Max))
  (return (+ _returnvalue 2.0) _returnvalue))

(fn `SimpleTrace`
  (returns (Initial :type "Vector Structure") (Final :type "Vector Structure"))
  (bind (_return_value_location _return_value_rotation) (`self.AnySocketTranform` "Muzzle"))
  (return _return_value_location (+ _return_value_location (* (`KismetMathLibrary.GetForwardVector` _return_value_rotation) 50000.0))))

(fn `SpreadTrace`
  (params (Initial :type "Vector Structure") (SpreadIntensity :type "Float (double-precision)"))
  (returns (Final :type "Vector Structure"))
  (bind _spread (`self.Spread`))
  (bind _returnvalue (`KismetMathLibrary.SelectFloat` (/ _spread 2.2) _spread (`/Game/GameContent/Blueprints/FPCharacter/FP_Character.ADS` (`self.Cast`))))
  (bind _returnvalue_2 (* _returnvalue SpreadIntensity))
  (return (+ Initial (`KismetMathLibrary.MakeVector` (`KismetMathLibrary.RandomFloatInRange` _returnvalue_2 _returnvalue) (`KismetMathLibrary.RandomFloatInRange` _returnvalue_2 _returnvalue) (`KismetMathLibrary.RandomFloatInRange` _returnvalue_2 _returnvalue)))))

(fn `UserConstructionScript`
  (`parent.UserConstructionScript`))