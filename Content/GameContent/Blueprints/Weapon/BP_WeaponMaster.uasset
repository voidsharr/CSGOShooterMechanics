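; BP_WeaponMaster is a weapon Blueprint, apparently a base class, with empty Fire and Reload events.
; AmmoCalc tops CurrentAmmo up toward Min, clamping TotalAmmo so the refill takes no more than the reserve holds.
; Helper functions return player 0's character cast to FP_Character and split a SkeletalMesh socket transform into location, rotation and scale.
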(event `Fire`)

(event `Reload`)

(fn `AmmoCalc`
  (locals (temp_Ammo :type Integer :default 0))
  (set `local.temp_Ammo` (`self.TotalAmmo`))
  (set `self.TotalAmmo` (`KismetMathLibrary.Clamp` (- (`self.TotalAmmo`) (- (`self.Min`) (`self.CurrentAmmo`))) 0 (`self.TotalAmmo`)))
  (set `self.CurrentAmmo` (+ (- (`local.temp_Ammo`) (`self.TotalAmmo`)) (`self.CurrentAmmo`)))
  (return))

(fn `AnySocketTranform`
  (params (InSocketName :type Name) (TransformSpace :type "ERelativeTransformSpace Enum" :default "RTS_World"))
  (returns (`Return Value Location` :type "Vector Structure") (`Return Value Rotation` :type "Rotator Structure") (`Return Value Scale` :type "Vector Structure"))
  (bind (_returnvalue_location _returnvalue_rotation _returnvalue_scale) (`KismetMathLibrary.BreakTransform` (`SceneComponent.GetSocketTransform` (`self.SkeletalMesh`) InSocketName TransformSpace)))
  (return _returnvalue_location _returnvalue_rotation _returnvalue_scale))

(fn `Cast`
  (returns (`AsFP Character` :type "/Game/GameContent/Blueprints/FPCharacter/FP_Character Object Reference"))
  (return (cast `/Game/GameContent/Blueprints/FPCharacter/FP_Character` (`GameplayStatics.GetPlayerCharacter` 0) :!pure true)))

(fn `UserConstructionScript`)